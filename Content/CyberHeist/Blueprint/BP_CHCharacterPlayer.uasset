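; BP_CHCharacterPlayer is the CyberHeist first-person player character Blueprint, adding left and right leaning.
; Each tilt input plays its own timeline on press and reverses it on release.
; Timeline tracks separately blend the relative transforms of the first-person camera and mesh between default and lean poses.
; A third timeline and control-type checks are disconnected and never run.
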(event Input|EnhancedActionEvents|EnhancedInputActionIA_LeftTilt
  (params (ActionValue :type Boolean) (ElapsedSeconds :type Float%20%28double-precision%29) (TriggeredSeconds :type Float%20%28double-precision%29) (InputAction :type Input%20Action%20Object%20Reference :default "/Game/CyberHeist/Input/Actions/IA_LeftTilt.IA_LeftTilt"))
  (:Started
    (bind (_direction _move_camera _guntrack) (Timeline|Timeline Play)
      (:Update
        (Transformation|SetRelativeTransform (Variables|Default|GetFirstPersonCamera) (Math|Transform|Lerp(Transform) (Variables|Default|GetCameraDefaultT) (Variables|Default|GetLeanLeftCameraT) _move_camera) false false)
        (Transformation|SetRelativeTransform (Variables|Default|GetFirstPersonMesh) (Math|Transform|Lerp(Transform) (Variables|Default|GetGunDefaultT) (Variables|Default|GetLeanLeftGunT) _guntrack) false false))))
  (:Completed
    (Timeline|Timeline Reverse)))

(event Input|EnhancedActionEvents|EnhancedInputActionIA_RightTilt
  (params (ActionValue :type Boolean) (ElapsedSeconds :type Float%20%28double-precision%29) (TriggeredSeconds :type Float%20%28double-precision%29) (InputAction :type Input%20Action%20Object%20Reference :default "/Game/CyberHeist/Input/Actions/IA_RightTilt.IA_RightTilt"))
  (:Started
    (bind (_direction _move_camera _guntrack) (Timeline|Timeline_0 Play)
      (:Update
        (Transformation|SetRelativeTransform (Variables|Default|GetFirstPersonCamera) (Math|Transform|Lerp(Transform) (Variables|Default|GetCameraDefaultT) (Variables|Default|GetLeanRightCameraT) _move_camera) false false)
        (Transformation|SetRelativeTransform (Variables|Default|GetFirstPersonMesh) (Math|Transform|Lerp(Transform) (Variables|Default|GetGunDefaultT) (Variables|Default|GetLeanRightGunT) _guntrack) false false))))
  (:Completed
    (Timeline|Timeline_0 Reverse)))

(event EventBeginPlay)

(event Collision|EventActorBeginOverlap
  (params (OtherActor :type Actor%20Object%20Reference)))

(event EventTick
  (params (DeltaSeconds :type Float%20%28single-precision%29)))

(fn ConstructionScript)