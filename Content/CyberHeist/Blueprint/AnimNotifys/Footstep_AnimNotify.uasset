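; Footstep anim notify for the player character, triggering the player's footstep logic and sound from animations.
; It casts the mesh owner to BP_Player, calls FootStep, then spawns the sound attached to the mesh, so other owners get neither.
; Volume is scaled down by the Mask_FootstepSound anim curve unless overridden.
; The footstep type is passed to the spawned sound as an integer parameter.
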(fn ReceivedNotify
  (params (MeshComp :type Skeletal%20Mesh%20Component%20Object%20Reference) (Animation :type Anim%20Sequence%20Base%20Object%20Reference) (EventReference :type Anim%20Notify%20Event%20Reference%20Structure%20%28by%20ref%29))
  (bind _returnvalue (Components|SkeletalMesh|GetAnimInstance MeshComp))
  (bind _sound (Variables|Default|GetSound))
  (Utilities|IsValid MeshComp
    (:Is%20Valid
      (Utilities|IsValid _returnvalue
        (:Is%20Valid
          (bind _asbp_player (Utilities|Casting|CastToBP_Player (Components|GetOwner MeshComp)))
          (Default|FootStep _asbp_player)
          (Utilities|IsValid _sound
            (:Is%20Valid
              (bind _returnvalue_2 (Audio|SpawnSoundAttached _sound MeshComp (Variables|Default|GetAttachPointName) "0, 0, 0" "0, 0, 0" "KeepRelativeOffset" true (select (Variables|Default|GetOverrideMaskCurve) (Variables|Default|GetVolumeMultiplier) (* (- 1.0 (Animation|Curves|GetCurveValue _returnvalue "Mask_FootstepSound")) (Variables|Default|GetVolumeMultiplier))) (Variables|Default|GetPitchMultiplier) 0.0 0 0))
              (Utilities|IsValid _returnvalue_2
                (:Is%20Valid
                  (Effects|Components|ParticleSystem|SetIntParameter _returnvalue_2 "FootstepType" (Math|Conversions|ToInteger(Byte) (Variables|Default|GetFootstepType)))
                  (return false))))))))))