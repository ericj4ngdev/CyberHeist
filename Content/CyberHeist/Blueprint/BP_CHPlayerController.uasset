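; Player controller for CyberHeist that owns the pause menu widget and toggles it with the P key.
; On BeginPlay the local controller creates the widget, adds it to the viewport collapsed and sets Game and UI input.
; TogglePasue flips IsPauseVisible, widget visibility and mouse cursor, switching between UI-only and game-only input.
; It does not pause the game itself.
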(event EventBeginPlay
  (bind _self self)
  (if (Pawn|IsLocalController)
    (bind _returnvalue (UserInterface|CreateWidget (Variables|Default|GetCHPauseWidgetClass) _self))
    (bind _output_get (Variables|Default|SetCHPauseWidget _returnvalue))
    (UserInterface|Viewport|AddtoViewport _output_get 0)
    (Input|SetInputModeGameandUI _self (Variables|Default|GetCHPauseWidget) "DoNotLock" false false)
    (Variables|Default|SetbShowMouseCursor false)
    (Widget|SetVisibility _output_get "Collapsed")))

(event EventTick
  (params (DeltaSeconds :type Float%20%28single-precision%29)))

(event Input|KeyboardEvents|P
  (params (Key :type Key%20Structure :default "None"))
  (:Pressed
    (CallFunction|TogglePasue (Variables|Default|GetCHPauseWidget) (Variables|Default|GetIsPauseVisible))))

(fn ConstructionScript)

(fn TogglePasue
  (params (타깃 :type Widget%20Object%20Reference) (Condition :type Boolean))
  (bind _self self)
  (if Condition
    (Variables|Default|SetIsPauseVisible false)
    (Widget|SetVisibility 타깃 "Hidden")
    (Input|SetInputModeGameOnly _self false)
    (Variables|Default|SetbShowMouseCursor false)
    (else
      (Variables|Default|SetIsPauseVisible true)
      (Widget|SetVisibility 타깃 "Visible")
      (Input|SetInputModeUIOnly _self 타깃 "DoNotLock" false)
      (Variables|Default|SetbShowMouseCursor true)))
  (return))