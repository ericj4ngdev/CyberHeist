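; Player Blueprint for CyberHeist that emits noise events at its own location, with itself as instigator, for AI hearing to pick up.
; The F key acts as a debug-style noisemaker, pairing a noise with a small explosion effect, quiet sound and printed message.
; FootStep emits a quieter noise and AnnounceLocation a range-limited one; neither event is called within this graph.
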(event Custom|Announce%20Location
  (Class|Actor|MakeNoise 1.0 self (Transformation|GetActorLocation) 2e+03 "None"))

(event Custom|FootStep
  (Class|Actor|MakeNoise 0.2 self (Transformation|GetActorLocation) 0.0 "None"))

(event EventBeginPlay)

(event Collision|EventActorBeginOverlap
  (params (OtherActor :type Actor%20Object%20Reference)))

(event EventTick
  (params (DeltaSeconds :type Float%20%28single-precision%29)))

(event Input|KeyboardEvents|F
  (params (Key :type Key%20Structure :default "None"))
  (bind _returnvalue (Transformation|GetActorLocation))
  (:Pressed
    (Class|Actor|MakeNoise 1.0 self _returnvalue 0.0 "None")
    (Effects|SpawnEmitteratLocation "/Game/Assets/MilitaryWeapSilver/FX/P_Grenade_Explosion_01.P_Grenade_Explosion_01" _returnvalue "0, 0, 0" "0.100000,0.100000,0.100000")
    (Audio|PlaySoundatLocation "/Game/Assets/MilitaryWeapSilver/Sound/RocketLauncher/Wavs/RocketLauncher_Explosion01.RocketLauncher_Explosion01" _returnvalue "0, 0, 0" 0.1 1.0 0.0 0 0 0 0)
    (Development|PrintString "Sound ")))

(fn ConstructionScript)