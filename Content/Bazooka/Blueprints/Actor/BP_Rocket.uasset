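; Rocket projectile actor for the bazooka that hands a homing target to its ProjectileMovement on BeginPlay and scales its scene component by a Scale variable at construction.
; Overlapping a BP_Target or BP_Target-Move spawns an enlarged explosion and destroys that target, but not the rocket.
; A Delay on Tick serves as the rocket's lifetime before it destroys itself.
; Pressing E activates its Niagara effect.
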(event EventBeginPlay
  (Variables|/Script/Engine.ProjectileMovementComponent|SetHomingTargetComponent (Variables|Default|GetProjectileMovement) (Variables|Default|GetHoming%20Target%20Component)))

(event Collision|EventActorBeginOverlap
  (params (OtherActor :type Actor%20Object%20Reference))
  (Utilities|FlowControl|Sequence
    (:then_0
      (bind _asbp_target (Utilities|Casting|CastToBP_Target OtherActor))
      (Effects|SpawnEmitteratLocation "/Game/Bazooka/VFX/P_Explosion.P_Explosion" (Transformation|GetActorLocation) "0, 0, 0" "10.000000,10.000000,10.000000")
      (Actor|DestroyActor _asbp_target))
    (:then_1
      (bind _asbp_target__move (Utilities|Casting|CastToBP_Target-Move OtherActor))
      (Effects|SpawnEmitteratLocation "/Game/Bazooka/VFX/P_Explosion.P_Explosion" (Transformation|GetActorLocation) "0, 0, 0" "10.000000,10.000000,10.000000")
      (Actor|DestroyActor _asbp_target__move))))

(event EventTick
  (params (DeltaSeconds :type Float%20%28single-precision%29))
  (Utilities|FlowControl|Delay 3e+01)
  (Actor|DestroyActor))

(event Input|KeyboardEvents|E
  (params (Key :type Key%20Structure :default "None"))
  (:Pressed
    (Components|Activation|Activate (Variables|Default|GetNiagara) true)))

(fn ConstructionScript
  (bind __scale (Variables|Default|Get%20Scale))
  (Transformation|SetWorldScale3D (Variables|Default|GetScene) (Math|Vector|MakeVector __scale __scale __scale)))