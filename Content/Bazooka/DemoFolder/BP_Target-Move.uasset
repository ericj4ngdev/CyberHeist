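; Moving target actor for the Bazooka demo that flies on its own with simplified aircraft motion.
; Each tick it moves along its forward vector at a thrust speed set on BeginPlay, with drag-smoothed slowdown and speed-mapped gravity.
; Interpolated yaw and roll take frame delta time as their input, so it keeps turning and banking, while the pitch function is never called.
; Any BP_Rocket that ends overlap with its Box is destroyed.
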(event OnComponentEndOverlap(Box)
  (params (OverlappedComponent :type Primitive%20Component%20Object%20Reference) (OtherActor :type Actor%20Object%20Reference) (OtherComp :type Primitive%20Component%20Object%20Reference) (OtherBodyIndex :type Integer))
  (bind _asbp_rocket (Utilities|Casting|CastToBP_Rocket OtherActor))
  (Actor|DestroyActor _asbp_rocket))

(event EventBeginPlay
  (Utilities|FlowControl|Sequence
    (:then_0
      (bind _output_get (Variables|Components|SetThrusSpeed (Variables|Default|GetMinThrusToNotfall)))
      (Variables|Components|SetCurrentSpeed _output_get))))

(event EventTick
  (params (DeltaSeconds :type Float%20%28single-precision%29))
  (Utilities|FlowControl|Sequence
    (:then_0
      (CallFunction|UpditePosichane DeltaSeconds))
    (:then_1
      (CallFunction|UpditeYaw (Utilities|Time|GetWorldDeltaSeconds) DeltaSeconds))
    (:then_2
      (CallFunction|UpditeRoll (Utilities|Time|GetWorldDeltaSeconds) DeltaSeconds))))

(fn ConstructionScript)

(fn UpditePosichane
  (params (DeltaSeconds :type Float%20%28single-precision%29))
  ;[1 1 1] CCS
  (Variables|Components|SetCurrentSpeed (select (< (Variables|Components|GetThrusSpeed) (Variables|Components|GetCurrentSpeed)) (Math|Interpolation|FInterpTo (Variables|Components|GetCurrentSpeed) (Variables|Components|GetThrusSpeed) DeltaSeconds (Variables|Components|GetDrag)) (Variables|Components|GetThrusSpeed)))
  ;[1 1 1] CNPBCS
  (LocalVariables|SetNewPosichane (* (Transformation|GetActorForwardVector) (* (Variables|Components|GetCurrentSpeed) DeltaSeconds)))
  ;[1 1 1] CAG
  (Variables|Components|SetApplieGravity (Math|Float|MapRangeClamped (Variables|Components|GetCurrentSpeed) 0.0 (Variables|Default|GetMinThrusToNotfall) (Variables|Components|GetGravity) 0.0))
  ;[1 1 1] UP
  (Transformation|AddActorWorldOffset (Math|Vector|MakeVector (.X (Math|Vector|BreakVector (LocalVariables|GetNewPosichane))) (.Y (Math|Vector|BreakVector (LocalVariables|GetNewPosichane))) (- (.Z (Math|Vector|BreakVector (LocalVariables|GetNewPosichane))) (* (Variables|Components|GetApplieGravity) DeltaSeconds)))))

(fn UpditeYaw
  (params (DeltaSeconds :type Float%20%28single-precision%29) (Yaw :type Float%20%28single-precision%29))
  (Variables|Components|SetTargetYaw Yaw)
  (bind _output_get (Variables|Components|SetCurrentYaw (Math|Interpolation|FInterpTo (Variables|Components|GetCurrentYaw) (Variables|Components|GetTargetYaw) DeltaSeconds 1e+01)))
  (Transformation|AddActorLocalRotation (Math|Rotator|MakeRotator 0.0 0.0 (* _output_get DeltaSeconds 1.2e+03)) false false))

(fn UpditePitch
  (params (DeltaSeconds :type Float%20%28single-precision%29) (Pitch :type Float%20%28single-precision%29))
  (Variables|Components|SetTargetPitch Pitch)
  (bind _output_get (Variables|Components|SetCurrentPitch (Math|Interpolation|FInterpTo (Variables|Components|GetCurrentPitch) (Variables|Components|GetTargetPitch) DeltaSeconds 1e+01)))
  (Transformation|AddActorLocalRotation (Math|Rotator|MakeRotator 0.0 (* _output_get DeltaSeconds 1e+02) 0.0) false false))

(fn UpditeRoll
  (params (DeltaSeconds :type Float%20%28single-precision%29) (Roll :type Float%20%28single-precision%29))
  (Variables|Components|SetTargetRoll Roll)
  (bind _output_get (Variables|Components|SetCurrentRoll (Math|Interpolation|FInterpTo (Variables|Components|GetCurrentRoll) (Variables|Components|GetTargetRoll) DeltaSeconds 1e+01)))
  (Transformation|AddActorLocalRotation (Math|Rotator|MakeRotator (* _output_get DeltaSeconds 1e+01) 0.0 0.0) false false))