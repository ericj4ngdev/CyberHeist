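; Game mode for the FPS starter pack that owns the player's HUD, death menu and circular progress widgets.
; On BeginPlay it shows the HUD, creates the other two widgets off-screen, unpauses and sets game-only input.
; HudDead pauses the game and swaps the HUD for the death menu with cursor and UI input.
; The Lola event plays a timeline that feeds the circular progress bar.
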(event Custom|Lola
  (bind _newtrack_0 (Timeline|Timeline_0 Play)
    (:Update
      (Default|ProgressCircular (Variables|Default|GetCircular) _newtrack_0))))

(event Custom|HudDead
  (bind _returnvalue (Game|GetPlayerController 0))
  (bind _deadwidget (Variables|Default|GetDeadWidget))
  (Game|SetGamePaused true)
  (Widget|RemovefromParent (Variables|Default|GetHud))
  (UserInterface|Viewport|AddtoViewport _deadwidget 0)
  (Variables|/Script/Engine.PlayerController|SetbShowMouseCursor _returnvalue true)
  (Input|SetInputModeGameandUI _returnvalue _deadwidget "DoNotLock" true false))

(event EventBeginPlay
  (bind _returnvalue (Game|GetPlayerController 0))
  (Utilities|FlowControl|Sequence
    (:then_0
      (bind _returnvalue_2 (UserInterface|CreateWidget "/Game/FpsStarterPack/System/WidgetBlueprint/WB_HudPlayer.WB_HudPlayer_C"))
      (bind _output_get (Variables|Default|SetHud _returnvalue_2))
      (UserInterface|Viewport|AddtoViewport _output_get 0))
    (:then_1
      (bind _returnvalue_3 (UserInterface|CreateWidget "/Game/FpsStarterPack/System/WeaponSystem/Blueprint/WB_CircularProgressBar.WB_CircularProgressBar_C"))
      (Variables|Default|SetCircular _returnvalue_3)
      (bind _returnvalue_4 (UserInterface|CreateWidget "/Game/FpsStarterPack/System/WidgetBlueprint/WB_DeadMenu.WB_DeadMenu_C"))
      (Variables|Default|SetDeadWidget _returnvalue_4))
    (:then_2
      (Game|SetGamePaused false)
      (Variables|/Script/Engine.PlayerController|SetbShowMouseCursor _returnvalue false)
      (Input|SetInputModeGameOnly _returnvalue false))))

(fn ConstructionScript)