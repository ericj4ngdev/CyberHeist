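; BP_Target is a shooting target actor that drops when its health runs out and rises again afterwards.
; AnyDamage and RadialDamage each subtract from Health and trigger the drop animation at zero or below.
; A timeline drives the Target's relative roll, with a three-second Delay on its Update pin leading to Reverse.
; Health is never reset here, so later hits trigger the drop again.
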(event Custom|dropAnimation
  (bind _newtrack_0 (Timeline|Timeline_0 Play)
    (:Update
      (Transformation|SetRelativeRotation (Variables|Default|Gettarget) (Math|Rotator|MakeRotator _newtrack_0 0.0 0.0) false false)
      (Utilities|FlowControl|Delay 3.0)
      (Timeline|Timeline_0 Reverse))))

(event EventBeginPlay)

(event Collision|EventActorBeginOverlap
  (params (OtherActor :type Actor%20Object%20Reference)))

(event Game|Damage|EventRadialDamage
  (params (DamageReceived :type Float%20%28single-precision%29) (DamageType :type Damage%20Type%20Object%20Reference) (Origin :type Vector :default "0, 0, 0") (HitInfo :type Hit%20Result%20Structure%20%28by%20ref%29) (InstigatedBy :type Controller%20Object%20Reference) (DamageCauser :type Actor%20Object%20Reference))
  (Variables|Default|SetHealth (- (Variables|Default|GetHealth) DamageReceived))
  (if (<= (Variables|Default|GetHealth) 0.0)
    (CallFunction|DropAnimation)))

(event EventTick
  (params (DeltaSeconds :type Float%20%28single-precision%29)))

(event Game|Damage|EventAnyDamage
  (params (Damage :type Float%20%28single-precision%29) (DamageType :type Damage%20Type%20Object%20Reference) (InstigatedBy :type Controller%20Object%20Reference) (DamageCauser :type Actor%20Object%20Reference))
  (Variables|Default|SetHealth (- (Variables|Default|GetHealth) Damage))
  (if (<= (Variables|Default|GetHealth) 0.0)
    (CallFunction|DropAnimation)))

(fn ConstructionScript)