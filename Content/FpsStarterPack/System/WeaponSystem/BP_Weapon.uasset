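; Base FPS weapon actor that the player picks up, fires, reloads, drops and sights through via camera view-target blends.
; Weapon state toggles physics and collision between dropped and equipped.
; FireLogic routes to shotgun, sniper or default hitscan shots from the camera, looping for auto and burst, with damage, tracers and camera shake.
; Reloads draw on reserve ammo, MultiGates cycle fire modes, and surface impact functions are unwired stubs.
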(event Custom|StartFire
  ;[1 0 0.5017] Fire
  (|FireLogic))

(event Custom|SightON
  ;[0 0.3281 0.0225 1 50] Sight
  (Game|Player|SetViewTargetwithBlend (Game|GetPlayerController 0) self 0.2 "VTBlend_Linear" 0.0 false))

(event Custom|InspectAnimation
  ;[0 0.3281 0.0225 1 50] inspect Animation
  (bind _returnvalue (Animation|Montage|MontagePlay (Components|SkeletalMesh|GetAnimInstance (Variables|/Script/Engine.Character|GetMesh (Game|GetPlayerCharacter 0))) (Variables|WeaponAnimations|GetAnimation_inspect) 1.0 "MontageLength" 0.0 true))
  (Utilities|FlowControl|Delay _returnvalue))

(event Custom|EquipAnimation
  ;[0 0.3281 0.0225 1 50] Equip Weapon Animation
  (bind _returnvalue (Animation|Montage|MontagePlay (Components|SkeletalMesh|GetAnimInstance (Variables|/Script/Engine.Character|GetMesh (Game|GetPlayerCharacter 0))) (Variables|WeaponAnimations|GetEquip) 1.0 "MontageLength" 0.0 true))
  (Utilities|FlowControl|Delay _returnvalue))

(event Custom|WeaponFireCustomShotgun
  ;[1 0 0.5017] Fire
  (|ShotgunFire))

(event Custom|modefire
  ;[0 1 0.811 1 50] ModeFire
  (if (not (Utilities|Enum|Equal(Enum) (Variables|WeaponConfig|GetSwitch%20Firing%20Modes) "NewEnumerator0"))
    (if (not (Utilities|Enum|Equal(Enum) (Variables|WeaponConfig|GetSwitch%20Firing%20Modes) "NewEnumerator1"))
      (if (not (Utilities|Enum|Equal(Enum) (Variables|WeaponConfig|GetSwitch%20Firing%20Modes) "NewEnumerator2"))
        (if (Utilities|Enum|Equal(Enum) (Variables|WeaponConfig|GetSwitch%20Firing%20Modes) "NewEnumerator3")
          (Utilities|FlowControl|MultiGate false true -1
            (:Out%200
              (Variables|Default|SetModeState "NewEnumerator1"))
            (:Out%201
              (Variables|Default|SetModeState "NewEnumerator0")))
          (elif (Utilities|Enum|Equal(Enum) (Variables|WeaponConfig|GetSwitch%20Firing%20Modes) "NewEnumerator4")
            (Utilities|FlowControl|MultiGate false true -1
              (:Out%200
                (Variables|Default|SetModeState "NewEnumerator2"))
              (:Out%201
                (Variables|Default|SetModeState "NewEnumerator0")))
            (elif (Utilities|Enum|Equal(Enum) (Variables|WeaponConfig|GetSwitch%20Firing%20Modes) "NewEnumerator5")
              (Utilities|FlowControl|MultiGate false true -1
                (:Out%200
                  (Variables|Default|SetModeState "NewEnumerator2"))
                (:Out%201
                  (Variables|Default|SetModeState "NewEnumerator1")))
              (elif (Utilities|Enum|Equal(Enum) (Variables|WeaponConfig|GetSwitch%20Firing%20Modes) "NewEnumerator6")
                (Utilities|FlowControl|MultiGate false true -1
                  (:Out%200
                    (Variables|Default|SetModeState "NewEnumerator2"))
                  (:Out%201
                    (Variables|Default|SetModeState "NewEnumerator1"))
                  (:Out%202
                    (Variables|Default|SetModeState "NewEnumerator0")))))))))))

(event Custom|WeaponFireCustomSniper
  ;[1 0 0.5017] Fire
  (|FireSniper))

(event Custom|WeaponRecoil
  (params (Pitch :type Float%20%28double-precision%29) (Yaw :type Float%20%28double-precision%29))
  (bind _returnvalue (Game|GetPlayerCharacter 0))
  (bind _returnvalue_2 (* Yaw 1.0))
  ;[0.8716 1 0 1 50] Recoil System
  (Pawn|Input|AddControllerPitchInput _returnvalue (select false (/ (* Pitch 1.0) 2.0) Pitch))
  (Pawn|Input|AddControllerYawInput _returnvalue (select false (/ _returnvalue_2 2.0) _returnvalue_2)))

(event Custom|SightOFF
  ;[0 0.3281 0.0225 1 50] Sight
  (Game|Player|SetViewTargetwithBlend (Game|GetPlayerController 0) (Game|GetPlayerCharacter 0) 0.2 "VTBlend_Linear" 0.0 false))

(event Custom|AnimationReloadWeapon
  ;[0 0.3281 0.0225 1 50] ReloadWeapon
  (Utilities|FlowControl|Sequence
    (:then_0
      (bind _weaponreloadanimation (Variables|WeaponAnimations|GetWeaponReloadAnimation)
        (:then
          (Animation|Montage|MontagePlay (Components|SkeletalMesh|GetAnimInstance (Variables|Default|GetSkeletalMesh)) _weaponreloadanimation 1.0 "MontageLength" 0.0 true))
        (:else)))
    (:then_1
      (bind _playerreloadanimation (Variables|WeaponAnimations|GetPlayerReloadAnimation)
        (:then
          (Animation|Montage|MontagePlay (Components|SkeletalMesh|GetAnimInstance (Variables|/Script/Engine.Character|GetMesh (Game|GetPlayerCharacter 0))) _playerreloadanimation 1.0 "MontageLength" 0.0 true))
        (:else)))))

(event Custom|Reload
  ;[1 0 0.07796 1 50] System Reload
  (if (== (Variables|WeaponConfig|GetMax%20Ammo) 0)
    (Development|PrintString "find ammors")
    (elif (== (Variables|Default|GetClipSize) (Variables|WeaponConfig|GetCurrentAmmo))
      (Development|PrintString "Full Ammor")
      (else
        (bind _output_get (Variables|Default|SetIsReloading? true))
        (if _output_get
          (CallFunction|WeaponReload)
          (Utilities|FlowControl|Delay 2.0)
          (Variables|Default|SetIsReloading? false))))))

(event Custom|Weapon%20Reload
  ;[1 0 0.07796 1 50] System Reload
  (if (not (Variables|Default|GetCanFire))
    (CallFunction|AnimationReloadWeapon)
    (if (not (Variables|WeaponConfig|GetCustomReload?))
      (if (> (Variables|WeaponConfig|GetMax%20Ammo) 0)
        (Variables|Default|SetNeededAmmo (- (Variables|Default|GetClipSize) (Variables|WeaponConfig|GetCurrentAmmo)))
        (if (<= (Variables|WeaponConfig|GetMax%20Ammo) (Variables|Default|GetNeededAmmo))
          (Variables|WeaponConfig|SetCurrentAmmo (+ (Variables|WeaponConfig|GetCurrentAmmo) (Variables|WeaponConfig|GetMax%20Ammo)))
          (Variables|WeaponConfig|SetMax%20Ammo 0)
          (else
            (Variables|WeaponConfig|SetMax%20Ammo (- (Variables|WeaponConfig|GetMax%20Ammo) (Variables|Default|GetNeededAmmo)))
            (Variables|WeaponConfig|SetCurrentAmmo (Variables|Default|GetClipSize))))))))

(event Custom|ReloadAnimationCustom
  ;[0 1 0.2384 1 50] BeginPlay
)

(event Custom|ShootingAnimation
  (bind _returnvalue (Game|GetPlayerCharacter 0))
  (bind _skeletalmesh (Variables|Default|GetSkeletalMesh))
  (bind _returnvalue_2 (Components|SkeletalMesh|GetAnimInstance _skeletalmesh))
  (bind _mesh (Variables|/Script/Engine.Character|GetMesh _returnvalue))
  (bind _returnvalue_3 (Components|SkeletalMesh|GetAnimInstance _mesh))
  ;[0 0.3281 0.0225 1 50] Shooting Animation
  (Utilities|FlowControl|Sequence
    (:then_0
      (if (Variables|Default|GetFullAuto?)
        (Animation|Montage|MontagePlay _returnvalue_3 (Variables|WeaponAnimations|GetPlayerShootingAniamtionFireFull) 1.0 "MontageLength" 0.0 true)
        (Variables|Default|SetIsShooting false)
        (else
          (bind _returnvalue_4 (Animation|Montage|MontagePlay _returnvalue_3 (Variables|WeaponAnimations|GetPlayerShootingAniamtion) 1.0 "MontageLength" 0.0 true))
          (Utilities|FlowControl|Delay _returnvalue_4)
          (Variables|Default|SetIsShooting false))))
    (:then_1
      (Utilities|IsValid _returnvalue_2
        (:Is%20Valid
          (Animation|Montage|MontagePlay _returnvalue_2 (Variables|WeaponAnimations|GetWeaponShootingAnimation) 1.0 "MontageLength" 0.0 true))))))

(event Custom|ReloadCustom
  ;[1 0.4363 0] ReloadCustom
  (if (not (== (Variables|WeaponConfig|GetCurrentAmmo) (Variables|Default|GetClipSize)))
    (if (>= (Variables|WeaponConfig|GetMax%20Ammo) 1)
      (Variables|WeaponConfig|SetCurrentAmmo (+ (Variables|WeaponConfig|GetCurrentAmmo) 1))
      (Variables|WeaponConfig|SetMax%20Ammo (- (Variables|WeaponConfig|GetMax%20Ammo) 1)))))

(event Custom|CheckAmmo
  ;[1 0 0.07796 1 50] System Reload
  (if (> (Variables|WeaponConfig|GetCurrentAmmo) 0)
    (Variables|Default|SetCan%20Shoot? true)
    (else
      (Variables|Default|SetCan%20Shoot? false))))

(event EventBeginPlay
  ;[0 1 0.2384 1 50] BeginPlay
  (Utilities|FlowControl|Sequence
    (:then_0
      (Private|SetWeaponState "NewEnumerator0"))
    (:then_1
      (bind _asbp_fpscharacter (Utilities|Casting|CastToBP_FPSCharacter (Game|GetPlayerCharacter 0)))
      (Variables|Default|SetCharacter _asbp_fpscharacter))
    (:then_2
      (Variables|Default|SetClipSize (Variables|WeaponConfig|GetCurrentAmmo)))))

(event EventRecoil
  (params (Pitch :type Float%20%28double-precision%29) (Yaw :type Float%20%28double-precision%29))
  ;[0.8716 1 0 1 50] Recoil System
  (CallFunction|WeaponRecoil Pitch Yaw))

(event EventInteract
  (params (Player :type BP%20Weapon%20Component%20Object%20Reference))
  ;[0 1 0.2259 1 50] Weapon State
  (Class|BPWeaponSystemInterface|PickUpWeapon(Message) Player self)
  (Private|SetWeaponState "NewEnumerator1"))

(fn ConstructionScript
  (|CallParentFunction)
  (Variables|Default|SetMaxAmmoDefault (Variables|WeaponConfig|GetMax%20Ammo))
  (Variables|Default|SetNameWe (Utilities|String|StringToName (Variables|WeaponConfig|GetName))))

(fn GetInteractionText
  (params (NewParam1 :type Text))
  (return "Pick Up"))

(fn GetInteractionTextAttach
  (return (Variables|Default|GetSkeletalMesh)))

(fn SetWeaponState
  (params (NewWeaponState :type E_WeaponState%20Enum :default "NewEnumerator0"))
  (bind _skeletalmesh (Variables|Default|GetSkeletalMesh))
  (bind _skeletalmesh_2 (Variables|Default|GetSkeletalMesh))
  (bind _output_get (Variables|Default|SetWeaponState NewWeaponState))
  (switch Utilities|FlowControl|Switch|SwitchonE_WeaponState _output_get
    (:NewEnumerator0
      (Collision|SetCollisionProfileName (Variables|Default|GetSphere) "OverlapAllDynamic" true :!class /Script/Engine.PrimitiveComponent)
      (Physics|SetSimulatePhysics _skeletalmesh_2 true)
      (Collision|SetCollisionProfileName _skeletalmesh_2 "WeaponDrop" true :!class /Script/Engine.PrimitiveComponent))
    (:NewEnumerator1
      (Collision|SetCollisionProfileName (Variables|Default|GetSphere) "NoCollision" true :!class /Script/Engine.PrimitiveComponent)
      (Physics|SetSimulatePhysics _skeletalmesh false)
      (Collision|SetCollisionProfileName _skeletalmesh "NoCollision" true :!class /Script/Engine.PrimitiveComponent)
      (Transformation|ResetRelativeTransform (Variables|Default|GetSkeletalMesh)))))

(fn Drop
  (Private|SetWeaponState "NewEnumerator0"))

(fn CheckFireMode
  (if (Variables|Default|GetFullAuto?)
    (CallFunction|FullAutoFire)
    (elif (Variables|Default|GetBurts?)
      (bind _counter (Utilities|FlowControl|DoN 2)
        (:Exit
          (CallFunction|BurstFire)
          (if (== _counter 2)
            _))))))

(fn CheckAmmoReturn
  (if (== (Variables|WeaponConfig|GetCurrentAmmo) (Variables|Default|GetClipSize))
    (bind _output_get (Variables|Default|SetIsAmmo? true :!label _label))
    (return _output_get)
    (elif (== (Variables|WeaponConfig|GetMax%20Ammo) 0)
      (goto _label))))

(fn StopMontageReload
  (params (Montage :type Anim%20Montage%20Object%20Reference))
  (Class|AnimInstance|MontagePause (Components|SkeletalMesh|GetAnimInstance (Variables|Default|GetSkeletalMesh)) Montage))

(fn BulletImpactSurface
  (params (Hit :type Hit%20Result%20Structure%20%28by%20ref%29) (Location :type Vector) (Rotation :type Rotator)))

(fn Decal
  (params (Hit :type Hit%20Result%20Structure%20%28by%20ref%29) (DecalSize :type Vector) (Location :type Vector) (Rotation :type Rotator) (LifeSpan :type Float%20%28double-precision%29)))

(fn BulletImpactSound
  (params (Hit :type Hit%20Result%20Structure%20%28by%20ref%29) (Location :type Vector) (VolumeMultiplier :type Float%20%28double-precision%29)))

(fn SwapAnimation
  (bind _returnvalue (Animation|Montage|MontagePlay (Components|SkeletalMesh|GetAnimInstance (Variables|/Script/Engine.Character|GetMesh (Game|GetPlayerCharacter 0))) (Variables|WeaponAnimations|GetSwap) 1.0 "MontageLength" 0.0 true))
  (return _returnvalue))

(fn PickingAmmo
  (if (< (Variables|WeaponConfig|GetMax%20Ammo) (Variables|Default|GetMaxAmmoDefault))
    (Variables|WeaponConfig|SetMax%20Ammo (Variables|Default|GetMaxAmmoDefault))
    (bind _output_get (Variables|Default|SetIsPickingAmmo? true))
    (return _output_get)
    (else
      (Variables|Default|SetIsPickingAmmo? false)
      (Development|PrintString "Full Ammor"))))

(event Custom|Burst%20Fire
  (CallFunction|CheckAmmo)
  (if (Variables|Default|GetCan%20Shoot?)
    (Utilities|FlowControl|Delay 0.05)
    (CallFunction|ShootingAnimation)
    (|Outputs) ; enters at BurstFire
    (else
      (Variables|Default|SetIsShooting? false))))

(event Custom|Full%20Auto%20Fire
  (if (Variables|Default|GetIsShooting?)
    (CallFunction|CheckAmmo)
    (if (Variables|Default|GetCan%20Shoot?)
      (Utilities|FlowControl|Delay (Variables|WeaponConfig|GetFireRate))
      (CallFunction|ShootingAnimation)
      (return)
      (else
        (Variables|Default|SetIsShooting? false)))))