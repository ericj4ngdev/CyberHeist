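; BP_BaseWeapon is a base weapon actor that shows a pickup prompt when an interactor comes within range.
; Entering range spawns a screen-space widget component at runtime, fills it with the weapon name and "pick up", and snaps it to the scene root.
; Leaving range destroys that component.
; Interact is an empty event, and the widget created on BeginPlay is separate from the displayed prompt.
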(event EventBeginPlay
  (bind _returnvalue (UserInterface|CreateWidget "/Game/FpsStarterPack/System/WeaponSystem/Blueprint/WB_InteractWidget.WB_InteractWidget_C"))
  (Variables|Default|SetWidget _returnvalue))

(event EventInteract
  (params (Player :type BP%20Weapon%20Component%20Object%20Reference)))

(event EventInteractRangeEntered
  (bind _returnvalue (Game|GetPlayerCharacter 0))
  (Utilities|IsValid _returnvalue
    (:Is%20Valid
      (Variables|Private|GetInteractWidgetComponent
        (:then)
        (:else
          (bind _returnvalue_2 (UserInterface|CreateWidget "/Game/FpsStarterPack/System/WeaponSystem/Blueprint/WB_InteractWidget.WB_InteractWidget_C" (.AsPlayer%20Controller (Utilities|Casting|CastToPlayerController (Pawn|GetController _returnvalue))) (Utilities|Text|ToText(Name) (Variables|Default|GetNameWe)) "pick up"))
          (bind _returnvalue_3 (AddComponent|AddWidgetComponent false))
          (bind _output_get (Variables|Private|SetInteractWidgetComponent _returnvalue_3))
          (UserInterface|SetWidget _output_get _returnvalue_2)
          (Class|WidgetComponent|SetWidgetSpace _output_get "Screen")
          (Class|WidgetComponent|SetDrawatDesiredSize _output_get true)
          (Collision|SetCollisionEnabled _output_get "NoCollision")
          (Transformation|AttachComponentToComponent _output_get (Private|GetInteractionTextAttach) "None" "SnapToTarget" "SnapToTarget" "SnapToTarget" true))))))

(event EventInteractRangeExited
  (bind _interactwidgetcomponent (Variables|Private|GetInteractWidgetComponent)
    (:then
      (Components|DestroyComponent _interactwidgetcomponent))
    (:else)))

(fn ConstructionScript)

(fn GetInteractionText
  (params (NewParam1 :type Text))
  (return NewParam1))

(fn GetInteractionTextAttach
  (return (Variables|Default|GetDefaultSceneRoot)))