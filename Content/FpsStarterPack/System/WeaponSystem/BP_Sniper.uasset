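; BP_Sniper is the sniper rifle weapon Blueprint, extending a parent class with scope aiming and a custom reload animation.
; Sight on shows the Lens component and blends the player's view target to the weapon actor itself; sight off hides it and blends back to the character.
; The custom reload event plays separate montages on the rifle's skeletal mesh and the player character's mesh together.
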(event EventBeginPlay
  (|CallParentFunction))

(event EventReloadAnimationCustom
  (Utilities|FlowControl|Sequence
    (:then_0
      (Animation|Montage|MontagePlay (Components|SkeletalMesh|GetAnimInstance (Variables|Default|GetSkeletalMesh)) "/Game/FpsStarterPack/System/WeaponSystem/WeaponMeshAndAnimations/Sniper/animations/A_Sniperreload_Montage.A_Sniperreload_Montage" 1.0 "MontageLength" 0.0 true))
    (:then_1
      (Animation|Montage|MontagePlay (Components|SkeletalMesh|GetAnimInstance (Variables|/Script/Engine.Character|GetMesh (Game|GetPlayerCharacter 0))) "/Game/FpsStarterPack/System/Player/Animations/SniperAnimations/A_reload_Montage.A_reload_Montage" 1.0 "MontageLength" 0.0 true))))

(event EventSightON
  (Rendering|SetVisibility (Variables|Default|GetLens) true false)
  (Game|Player|SetViewTargetwithBlend (Game|GetPlayerController 0) self 0.2 "VTBlend_Linear" 0.0 false))

(event EventSightOFF
  (Rendering|SetVisibility (Variables|Default|GetLens) false false)
  (Game|Player|SetViewTargetwithBlend (Game|GetPlayerController 0) (Game|GetPlayerCharacter 0) 0.2 "VTBlend_Linear" 0.0 false))

(fn ConstructionScript
  (|CallParentFunction))