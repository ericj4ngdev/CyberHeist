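; BP_Health is a health pickup actor for the FPS starter pack's weapon system.
; When its Sphere component overlaps a BP_FPSCharacter whose Health is below full, it sets Health directly to the maximum and destroys itself.
; A character already at full health leaves the pickup in place.
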(event OnComponentBeginOverlap(Sphere)
  (params (OverlappedComponent :type Primitive%20Component%20Object%20Reference) (OtherActor :type Actor%20Object%20Reference) (OtherComp :type Primitive%20Component%20Object%20Reference) (OtherBodyIndex :type Integer) (bFromSweep :type Boolean) (SweepResult :type Hit%20Result%20Structure%20%28by%20ref%29))
  (bind _asbp_fpscharacter (Utilities|Casting|CastToBP_FPSCharacter OtherActor))
  (if (< (Variables|/Game/FpsStarterPack/System/Player/BP_FPSCharacter.BP_FPSCharacter_C|GetHealth _asbp_fpscharacter) 1e+02)
    (Variables|/Game/FpsStarterPack/System/Player/BP_FPSCharacter.BP_FPSCharacter_C|SetHealth _asbp_fpscharacter 1e+02)
    (Actor|DestroyActor)))

(event Collision|EventActorBeginOverlap
  (params (OtherActor :type Actor%20Object%20Reference))
  (|CallParentFunction OtherActor) ; This node is disabled and will not be called.\nDrag off pins to build functionality.
)

(event EventBeginPlay
  (|CallParentFunction) ; This node is disabled and will not be called.\nDrag off pins to build functionality.
)

(fn ConstructionScript
  (|CallParentFunction))