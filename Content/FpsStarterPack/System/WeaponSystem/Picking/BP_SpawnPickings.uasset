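; BP_SpawnPickings is a spawner in the weapon system's picking folder that keeps an actor of a configurable class present in the level.
; Every Tick it searches the whole world for that class and, when none exist, starts a five-second Delay.
; After the delay it spawns one at a random point within the Box component's bounds, with zero rotation and unit scale.
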(event EventBeginPlay)

(event Collision|EventActorBeginOverlap
  (params (OtherActor :type Actor%20Object%20Reference)))

(event EventTick
  (params (DeltaSeconds :type Float%20%28single-precision%29))
  (bind _box (Variables|Default|GetBox))
  (bind (_origin _boxextent) (Collision|GetComponentBounds _box))
  (bind _outactors (Actor|GetAllActorsOfClass (Variables|Default|GetSpawnActor)))
  (if (<= (Utilities|Array|Length _outactors) 0)
    (Utilities|FlowControl|Delay 5.0)
    (Game|SpawnActorfromClass (Variables|Default|GetSpawnActor) (Math|Transform|MakeTransform (Math|Random|RandomPointinBoundingBox _origin _boxextent)) "Undefined" "SelectDefaultAtRuntime" 0 0)))

(fn ConstructionScript)