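; BP_Ammo is an ammo pickup for the FPS weapon system.
; When an actor overlaps its Sphere component, it casts to BP_FPSCharacter and calls GetAmmo on that character's weapon component.
; The pickup destroys itself only if GetAmmo returns true, leaving the ammo logic to the weapon component.
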(event OnComponentBeginOverlap(Sphere)
  (params (OverlappedComponent :type Primitive%20Component%20Object%20Reference) (OtherActor :type Actor%20Object%20Reference) (OtherComp :type Primitive%20Component%20Object%20Reference) (OtherBodyIndex :type Integer) (bFromSweep :type Boolean) (SweepResult :type Hit%20Result%20Structure%20%28by%20ref%29))
  (bind _asbp_fpscharacter (Utilities|Casting|CastToBP_FPSCharacter OtherActor))
  (bind _ispicking_ (Default|GetAmmo (Variables|/Game/FpsStarterPack/System/Player/BP_FPSCharacter.BP_FPSCharacter_C|GetBP_WeaponComponent _asbp_fpscharacter)))
  (if _ispicking_
    (Actor|DestroyActor)))

(event EventBeginPlay
  (|CallParentFunction) ; This node is disabled and will not be called.\nDrag off pins to build functionality.
)

(event Collision|EventActorBeginOverlap
  (params (OtherActor :type Actor%20Object%20Reference))
  (|CallParentFunction OtherActor))

(event EventTick
  (params (DeltaSeconds :type Float%20%28single-precision%29))
  (|CallParentFunction DeltaSeconds) ; This node is disabled and will not be called.\nDrag off pins to build functionality.
)

(fn ConstructionScript
  (|CallParentFunction))