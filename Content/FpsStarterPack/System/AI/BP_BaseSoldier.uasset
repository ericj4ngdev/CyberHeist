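; Base AI soldier character for an FPS, with health HUD, rifle or pistol, and crouched cover.
; BeginPlay spawns and attaches the configured weapon; AIAttack and StopAttack control looping fire timers.
; Shots are noise-reporting line traces with difficulty-based random yaw spread, and empty clips reload from reserve ammo.
; Damage plays random hit reactions; death ragdolls the body and destroys the weapon (pickup spawning is unwired), then the actor.
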(event Custom|EnterCover
  ;[1 0.3154 0.01179] going into cover
  (Variables|Default|SetIsCover true)
  (Character|Crouch))

(event Custom|StopAttack
  ;[1 0.1913 0.001031] Stop Attack
  (if (Variables|Default|GetIsEquip)
    (if (.Isvalid_Rifle (Utilities|CheckWeapons))
      (Utilities|Time|ClearandInvalidateTimerbyHandle (Variables|Default|GetRifleTimer))
      (Variables|Default|SetIsEnableCombatSight false))
    (elif (Variables|Default|GetIsEquipPistol)
      (if (.Isvalid_pistol (Utilities|CheckWeapons))
        (Utilities|Time|ClearandInvalidateTimerbyHandle (Variables|Default|GetPistolTimer))
        (Variables|Default|SetIsEnableCombatSight false)))))

(event Custom|Reloading
  ;[1 0.005986 0.6387] Reload Weapon
  (Variables|Default|SetIsReload true)
  (Animation|Montage|MontagePlay (Components|SkeletalMesh|GetAnimInstance (Variables|Character|GetMesh)) "/Game/FpsStarterPack/Demo/AnimationsAI/AnimationMontage/A_ReloadRifleHipMontage.A_ReloadRifleHipMontage" 1.0 "Duration" 0.0 true)
  (CallFunction|Reload)
  (Utilities|FlowControl|Delay 2.3)
  (Variables|Default|SetIsReload false))

(event EventBeginPlay
  ;[1 0.9316 0] Begin Play
  (Utilities|FlowControl|Sequence
    (:then_0
      ;[0 0.04887 1] Get AI HUD
      (Variables|Default|SetCurrentHealth (Utilities|Struct|BreakS_StatusSoldier (Variables|AllConfigSoldier|GetStatusSoldier)))
      (bind _aswb_aihud (Utilities|Casting|CastToWB_AIHUD (UserInterface|GetUserWidgetObject (Variables|Default|GetWidget))))
      (Variables|/Game/FpsStarterPack/System/AI/HUD/WB_AIHUD.WB_AIHUD_C|Setowner _aswb_aihud self)
      (Variables|Default|Sethud _aswb_aihud))
    (:then_1
      ;[0 0.08696 1] Spawn Weapon
      (CallFunction|SpawnWeapon))
    (:then_2
      (Rendering|SetVisibility (Variables|Default|GetWidget) (Utilities|Struct|BreakS_StatusSoldier (Variables|AllConfigSoldier|GetStatusSoldier)) false))))

(event EventAIAttack
  ;[1 0.1422 0] AI Attack
  (if (Variables|Default|GetIsEquip)
    (if (.Isvalid_Rifle (Utilities|CheckWeapons))
      (CallFunction|Shooting)
      (bind _returnvalue (Utilities|Time|SetTimerbyFunctionName 0 "Shooting" (Utilities|Struct|BreakS_WeaponItemType (Variables|/Game/FpsStarterPack/System/AI/Weapons/BP_BaseWeapon.BP_BaseWeapon_C|GetItemInfo (Variables|Default|GetBP_rifle))) true))
      (Variables|Default|SetRifleTimer _returnvalue)
      (Variables|Default|SetIsEnableCombatSight true))
    (elif (Variables|Default|GetIsEquipPistol)
      (if (.Isvalid_pistol (Utilities|CheckWeapons))
        (CallFunction|Shooting)
        (bind _returnvalue_2 (Utilities|Time|SetTimerbyFunctionName 0 "Shooting" (Utilities|Struct|BreakS_WeaponItemType (Variables|/Game/FpsStarterPack/System/AI/Weapons/BP_BaseWeapon.BP_BaseWeapon_C|GetItemInfo (Variables|Default|GetBP_pistol))) true))
        (Variables|Default|SetPistolTimer _returnvalue_2)
        (Variables|Default|SetIsEnableCombatSight true)))))

(event Game|Damage|EventAnyDamage
  (params (Damage :type Float%20%28single-precision%29) (DamageType :type Damage%20Type%20Object%20Reference) (InstigatedBy :type Controller%20Object%20Reference) (DamageCauser :type Actor%20Object%20Reference))
  (bind _widget (Variables|Default|GetWidget))
  (bind _mesh (Variables|Character|GetMesh))
  ;[0 1 0.05499] Damage
  ;;[0 0.1617 1] Animation Reaction
  (CallFunction|HitReaction)
  (Variables|Default|SetCurrentHealth (- (Variables|Default|GetCurrentHealth) (/ Damage 1e+02)))
  (if (<= (Variables|Default|GetCurrentHealth) 0.0)
    (Utilities|IsValid _widget
      (:Is%20Valid
        (Rendering|SetVisibility _widget false false)
        ;;[0 0.03912 1] Ragdoll
        (Physics|SetSimulatePhysics (Variables|Character|GetMesh) true)
        (Collision|SetCollisionEnabled _mesh "PhysicsOnly")
        (Collision|SetCollisionProfileName _mesh "Block All" true :!class /Script/Engine.PrimitiveComponent)
        (Collision|SetCollisionEnabled (Variables|Collision|GetCapsuleComponent) "NoCollision")
        ;;;[1 0.09597 0] Drop Weapon
        (CallFunction|DropWeapon)
        (Utilities|FlowControl|Delay 3.0)
        (Actor|DestroyActor)))))

(fn ConstructionScript
  (Variables|AllConfigSoldier|SetStatusSoldier (Utilities|Struct|MakeS_StatusSoldier (.health (Variables|AllConfigSoldier|GetStatusSoldier)) (.healthprogressbar (Variables|AllConfigSoldier|GetStatusSoldier)) (.spawnweapon (Variables|AllConfigSoldier|GetStatusSoldier)) (.dificultyai (Variables|AllConfigSoldier|GetStatusSoldier)))))

(fn SpawnWeapon
  (bind _mesh (Variables|Character|GetMesh))
  (switch Utilities|FlowControl|Switch|SwitchonE_WeaponType (Utilities|Struct|BreakS_StatusSoldier (Variables|AllConfigSoldier|GetStatusSoldier))
    (:NewEnumerator1
      ;[0 0.1803 1] Spawn Rifle
      (bind _returnvalue (Game|SpawnActorfromClass "/Game/FpsStarterPack/System/AI/Weapons/BP_AIRifle.BP_AIRifle_C" (Transformation|GetSocketTransform (Variables|Character|GetMesh) "hand_rSocket" "RTS_World") "Undefined" "OverrideRootScale" 0 0))
      (bind _output_get (Variables|Default|SetBP_rifle _returnvalue))
      (Variables|Default|SetCurrentWeapon _output_get)
      (Transformation|AttachComponentToComponent _output_get _mesh "hand_rSocket" "SnapToTarget" "SnapToTarget" "SnapToTarget" true)
      (Variables|Default|SetIsEquip true))
    (:NewEnumerator2
      ;[1 0 0.2228] Spawn Pistol
      (bind _returnvalue_2 (Game|SpawnActorfromClass "/Game/FpsStarterPack/System/AI/Weapons/BP_AIPistol.BP_AIPistol_C" (Transformation|GetSocketTransform (Variables|Character|GetMesh) "hand_rSocket" "RTS_World") "Undefined" "OverrideRootScale" 0 0))
      (bind _output_get_2 (Variables|Default|SetBP_pistol _returnvalue_2))
      (Variables|Default|SetCurrentWeapon _output_get_2)
      (Transformation|AttachComponentToComponent _output_get_2 _mesh "hand_rSocket" "SnapToTarget" "SnapToTarget" "SnapToTarget" true)
      (Variables|Default|SetIsEquipPistol true))))

(fn Shooting
  (bind (_start _end) (Utilities|LineTraceRifle))
  (bind (_start_2 _end_2) (Utilities|LineTracePistol))
  (bind _bp_rifle (Variables|Default|GetBP_rifle))
  (bind _bp_pistol (Variables|Default|GetBP_pistol))
  (bind _muzzle (Variables|/Game/FpsStarterPack/System/AI/Weapons/BP_BaseWeapon.BP_BaseWeapon_C|GetMuzzle _bp_rifle))
  (bind _muzzle_2 (Variables|/Game/FpsStarterPack/System/AI/Weapons/BP_BaseWeapon.BP_BaseWeapon_C|GetMuzzle _bp_pistol))
  (bind _returnvalue (Transformation|GetWorldLocation _muzzle_2))
  (bind _returnvalue_2 (Transformation|GetWorldLocation _muzzle))
  ;[0.021 0 1] Fire RIfle
  (if (Variables|Default|GetIsEquip)
    (if (.Isvalid_Rifle (Utilities|CheckWeapons))
      (if (not (or (Variables|Default|GetIsReload) (Variables|Default|GetIsDropWeapon)))
        ;[0 1 0.8916] Check Ammo
        (if (> (Utilities|Struct|BreakS_WeaponItemType (Variables|/Game/FpsStarterPack/System/AI/Weapons/BP_BaseWeapon.BP_BaseWeapon_C|GetItemInfo (Variables|Default|GetBP_rifle))) 0)
          ;[1 0.007764 0] Animation Fire
          (Animation|Montage|MontagePlay (Components|SkeletalMesh|GetAnimInstance (Variables|Character|GetMesh)) "/Game/FpsStarterPack/Demo/AnimationsAI/AnimationMontage/A_FireRifleIronsightsMontage.A_FireRifleIronsightsMontage" 1.0 "MontageLength" 0.0 true)
          (Math|Integer|DecrementInt (Utilities|Struct|BreakS_WeaponItemType (Variables|/Game/FpsStarterPack/System/AI/Weapons/BP_BaseWeapon.BP_BaseWeapon_C|GetItemInfo (Variables|Default|GetBP_rifle)))
            (:%20%20
              ;[0.02277 0.047 1] Effect Muzzle
              (Effects|SpawnEmitteratLocation 0 (Transformation|GetSocketLocation (Variables|/Game/FpsStarterPack/System/AI/Weapons/BP_BaseWeapon.BP_BaseWeapon_C|GetMuzzle (Variables|Default|GetBP_rifle)) "None"))
              ;[0 1 0.334] Play Sound Weapon
              (Audio|PlaySoundatLocation 0 _returnvalue_2 "0, 0, 0" 1.0 1.0 0.0 0 0 0 0)
              (Class|AISenseHearing|ReportNoiseEvent _returnvalue_2 1.0 self 0.0 "Noise")
              (bind (_outhit _returnvalue_3) (Collision|LineTraceByChannel _start _end "TraceTypeQuery1" true (Utilities|Array|MakeArray self) "None"))
              (if _returnvalue_3
                ;[1 0 0.7629] Effect Impact
                (Effects|SpawnEmitteratLocation 0 (.ImpactPoint (Collision|BreakHitResult _outhit)))
                ;[0 1 0.156] Damage Weapon
                (if (== (.HitActor (Collision|BreakHitResult _outhit)) (Game|GetPlayerCharacter 0))
                  (Game|Damage|ApplyDamage (.HitActor (Collision|BreakHitResult _outhit)) 1e+01 0 self)))))
          (elif (== (Utilities|Struct|BreakS_WeaponItemType (Variables|/Game/FpsStarterPack/System/AI/Weapons/BP_BaseWeapon.BP_BaseWeapon_C|GetItemInfo (Variables|Default|GetBP_rifle))) 0)
            (if (not (== (Utilities|Struct|BreakS_WeaponItemType (Variables|/Game/FpsStarterPack/System/AI/Weapons/BP_BaseWeapon.BP_BaseWeapon_C|GetItemInfo (Variables|Default|GetBP_rifle))) 0))
              (CallFunction|Reloading))))))
    (else
      ;[0 0.123 1] Fire Pistol
      (if (Variables|Default|GetIsEquipPistol)
        (if (.Isvalid_pistol (Utilities|CheckWeapons))
          (if (Variables|Default|GetIsEnablecombat)
            (if (not (or (Variables|Default|GetIsReload) (Variables|Default|GetIsDropWeapon)))
              ;[0 1 0.7793] Check Ammo
              (if (> (Utilities|Struct|BreakS_WeaponItemType (Variables|/Game/FpsStarterPack/System/AI/Weapons/BP_BaseWeapon.BP_BaseWeapon_C|GetItemInfo (Variables|Default|GetBP_pistol))) 0)
                ;[1 0.007764 0] Animation Fire
                (Animation|Montage|MontagePlay (Components|SkeletalMesh|GetAnimInstance (Variables|Character|GetMesh)) "/Game/FpsStarterPack/Demo/AnimationsAI/AnimationMontage/A_FireRifleIronsightsMontage.A_FireRifleIronsightsMontage" 1.0 "MontageLength" 0.0 true)
                (Math|Integer|DecrementInt (Utilities|Struct|BreakS_WeaponItemType (Variables|/Game/FpsStarterPack/System/AI/Weapons/BP_BaseWeapon.BP_BaseWeapon_C|GetItemInfo (Variables|Default|GetBP_pistol)))
                  (:%20%20
                    ;[0 0.03793 1] Effect Muzzle
                    (Effects|SpawnEmitteratLocation 0 (Transformation|GetSocketLocation (Variables|/Game/FpsStarterPack/System/AI/Weapons/BP_BaseWeapon.BP_BaseWeapon_C|GetMuzzle (Variables|Default|GetBP_pistol)) "None"))
                    ;[0 1 0.2948] Play Sound Weapon
                    (Audio|PlaySoundatLocation 0 _returnvalue "0, 0, 0" 1.0 1.0 0.0 0 0 0 0)
                    (Class|AISenseHearing|ReportNoiseEvent _returnvalue 1.0 self 0.0 "Noise")
                    (bind (_outhit_2 _returnvalue_4) (Collision|LineTraceByChannel _start_2 _end_2 "TraceTypeQuery1" true (Utilities|Array|MakeArray self) "None"))
                    (if _returnvalue_4
                      ;[1 0 0.8789] Effect Impact
                      (Effects|SpawnEmitteratLocation 0 (.ImpactPoint (Collision|BreakHitResult _outhit_2)))
                      ;[0 1 0.03587] Damage Weapon
                      (Game|Damage|ApplyDamage (.HitActor (Collision|BreakHitResult _outhit_2)) 1e+01 0 self))))
                (elif (== (Utilities|Struct|BreakS_WeaponItemType (Variables|/Game/FpsStarterPack/System/AI/Weapons/BP_BaseWeapon.BP_BaseWeapon_C|GetItemInfo (Variables|Default|GetBP_pistol))) 0)
                  (if (not (== (Utilities|Struct|BreakS_WeaponItemType (Variables|/Game/FpsStarterPack/System/AI/Weapons/BP_BaseWeapon.BP_BaseWeapon_C|GetItemInfo (Variables|Default|GetBP_pistol))) 0))
                    (CallFunction|Reloading)))))))))))

(fn Reload
  (bind _bp_rifle (Variables|Default|GetBP_rifle))
  (bind _bp_rifle_2 (Variables|Default|GetBP_rifle))
  (bind _bp_rifle_3 (Variables|Default|GetBP_rifle))
  (bind _bp_rifle_4 (Variables|Default|GetBP_rifle))
  (bind _bp_pistol (Variables|Default|GetBP_pistol))
  (bind _bp_pistol_2 (Variables|Default|GetBP_pistol))
  (bind _bp_pistol_3 (Variables|Default|GetBP_pistol))
  (bind _bp_pistol_4 (Variables|Default|GetBP_pistol))
  (bind _iteminfo (Variables|/Game/FpsStarterPack/System/AI/Weapons/BP_BaseWeapon.BP_BaseWeapon_C|GetItemInfo _bp_rifle))
  (bind _iteminfo_2 (Variables|/Game/FpsStarterPack/System/AI/Weapons/BP_BaseWeapon.BP_BaseWeapon_C|GetItemInfo _bp_rifle_2))
  (bind _iteminfo_3 (Variables|/Game/FpsStarterPack/System/AI/Weapons/BP_BaseWeapon.BP_BaseWeapon_C|GetItemInfo _bp_rifle_3))
  (bind _iteminfo_4 (Variables|/Game/FpsStarterPack/System/AI/Weapons/BP_BaseWeapon.BP_BaseWeapon_C|GetItemInfo _bp_rifle_4))
  (bind _iteminfo_5 (Variables|/Game/FpsStarterPack/System/AI/Weapons/BP_BaseWeapon.BP_BaseWeapon_C|GetItemInfo _bp_pistol))
  (bind _iteminfo_6 (Variables|/Game/FpsStarterPack/System/AI/Weapons/BP_BaseWeapon.BP_BaseWeapon_C|GetItemInfo _bp_pistol_2))
  (bind _iteminfo_7 (Variables|/Game/FpsStarterPack/System/AI/Weapons/BP_BaseWeapon.BP_BaseWeapon_C|GetItemInfo _bp_pistol_3))
  (bind _iteminfo_8 (Variables|/Game/FpsStarterPack/System/AI/Weapons/BP_BaseWeapon.BP_BaseWeapon_C|GetItemInfo _bp_pistol_4))
  (bind (_currentammo _clipsize) (Utilities|Struct|BreakS_WeaponItemType _iteminfo))
  (bind _maxammo (Utilities|Struct|BreakS_WeaponItemType _iteminfo_3))
  (bind (_currentammo_2 _maxammo_2) (Utilities|Struct|BreakS_WeaponItemType _iteminfo_2))
  (bind (_currentammo_3 _clipsize_2) (Utilities|Struct|BreakS_WeaponItemType _iteminfo_5))
  (bind _maxammo_3 (Utilities|Struct|BreakS_WeaponItemType _iteminfo_7))
  (bind (_currentammo_4 _maxammo_4) (Utilities|Struct|BreakS_WeaponItemType _iteminfo_6))
  (if (Variables|Default|GetIsEquip)
    (if (.Isvalid_Rifle (Utilities|CheckWeapons))
      ;[1 0.1235 0.1732] Reload Rifle
      (if (> (Utilities|Struct|BreakS_WeaponItemType (Variables|/Game/FpsStarterPack/System/AI/Weapons/BP_BaseWeapon.BP_BaseWeapon_C|GetItemInfo (Variables|Default|GetBP_rifle))) 0)
        (Variables|Default|SetNeededAmmo (- _clipsize _currentammo))
        (if (<= _maxammo (Variables|Default|GetNeededAmmo))
          (Utilities|Struct|SetmembersinS_WeaponItemType _iteminfo_4 (+ _currentammo_2 _maxammo_2))
          (Utilities|Struct|SetmembersinS_WeaponItemType _iteminfo_4)
          (else
            (Utilities|Struct|SetmembersinS_WeaponItemType _iteminfo_4 (- _maxammo (Variables|Default|GetNeededAmmo)))
            (Utilities|Struct|SetmembersinS_WeaponItemType _iteminfo_4 (Utilities|Struct|BreakS_WeaponItemType (Variables|/Game/FpsStarterPack/System/AI/Weapons/BP_BaseWeapon.BP_BaseWeapon_C|GetItemInfo (Variables|Default|GetBP_rifle))))))))
    (elif (Variables|Default|GetIsEquipPistol)
      (if (.Isvalid_pistol (Utilities|CheckWeapons))
        ;[0.9934 1 0.02968] Reload Pistol
        (if (> (Utilities|Struct|BreakS_WeaponItemType (Variables|/Game/FpsStarterPack/System/AI/Weapons/BP_BaseWeapon.BP_BaseWeapon_C|GetItemInfo (Variables|Default|GetBP_pistol))) 0)
          (Variables|Default|SetNeededAmmo (- _clipsize_2 _currentammo_3))
          (if (<= _maxammo_3 (Variables|Default|GetNeededAmmo))
            (Utilities|Struct|SetmembersinS_WeaponItemType _iteminfo_8 (+ _currentammo_4 _maxammo_4))
            (Utilities|Struct|SetmembersinS_WeaponItemType _iteminfo_8)
            (else
              (Utilities|Struct|SetmembersinS_WeaponItemType _iteminfo_8 (- _maxammo_3 (Variables|Default|GetNeededAmmo)))
              (Utilities|Struct|SetmembersinS_WeaponItemType _iteminfo_8 (Utilities|Struct|BreakS_WeaponItemType (Variables|/Game/FpsStarterPack/System/AI/Weapons/BP_BaseWeapon.BP_BaseWeapon_C|GetItemInfo (Variables|Default|GetBP_pistol)))))))))))

(fn DropWeapon
  (if (.Current%20Rifle (Utilities|CheckWeapons))
    (if (or (Variables|Default|GetIsEquip) (Variables|Default|GetSwagRifle))
      ;[0 0.1503 1] Drop Rifle
      (Variables|Default|SetIsDropWeapon true)
      (Actor|DestroyActor (Variables|Default|GetBP_rifle))
      (Variables|Default|SetCurrentWeapon 0)
      (Variables|Default|SetIsEquip false)
      (Variables|Default|SetIsWeaponEquip false)
      (Variables|Default|SetSwagRifle false)
      (else
        (Actor|DestroyActor (Variables|Default|GetBP_rifle))))
    (else
      ;[1 0.9505 0.1506] Drop pistol
      (if (.Current%20Pistol (Utilities|CheckWeapons))
        (if (or (Variables|Default|GetIsEquipPistol) (Variables|Default|GetSwagpistol))
          (Variables|Default|SetIsDropWeapon true)
          (Actor|DestroyActor (Variables|Default|GetBP_pistol))
          (Variables|Default|SetCurrentWeapon 0)
          (Variables|Default|SetIsEquipPistol false)
          (Variables|Default|SetIsWeaponEquip false)
          (Variables|Default|SetSwagpistol false)
          (else
            (Actor|DestroyActor (Variables|Default|GetBP_pistol))))))))

(fn HitReaction
  (switch int (Math|Random|RandomIntegerinRange 0 3)
    (:0
      ;[0.05098 0.01223 1] Animation Hit Reaction
      (Animation|PlayAnimMontage "/Game/FpsStarterPack/Demo/AnimationsAI/AnimationMontage/A_HitReact1Montage.A_HitReact1Montage" 1.0 "None"))
    (:1
      (Animation|PlayAnimMontage "/Game/FpsStarterPack/Demo/AnimationsAI/AnimationMontage/A_HitReact2Montage.A_HitReact2Montage" 1.0 "None"))
    (:2
      (Animation|PlayAnimMontage "/Game/FpsStarterPack/Demo/AnimationsAI/AnimationMontage/A_HitReact3Montage.A_HitReact3Montage" 1.0 "None"))
    (:3
      (Animation|PlayAnimMontage "/Game/FpsStarterPack/Demo/AnimationsAI/AnimationMontage/A_HitReact4Montage.A_HitReact4Montage" 1.0 "None"))))