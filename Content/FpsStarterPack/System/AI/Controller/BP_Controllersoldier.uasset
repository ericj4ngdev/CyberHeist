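; AI controller for soldier enemies that randomly runs either the courageous or shooting-cover behavior tree on BeginPlay.
; Perception updates about the player are read by stimulus array index as sight, hearing or damage, setting CanSeePlayer, Investigate and TargetLocation on the blackboard.
; Noise-tagged stimuli from other BP_BaseSoldier actors also write Investigate and TargetLocation.
; CanSeePlayer is only ever set true here, never cleared.
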(event OnTargetPerceptionUpdated(AIPerceptionSoldier)
  (params (Actor :type Actor%20Object%20Reference) (Stimulus :type AI%20Stimulus%20Structure))
  (bind (_age _expirationage _strength _stimuluslocation _receiverlocation _tag _bsuccessfullysensed) (Utilities|Struct|BreakAIStimulus Stimulus))
  ;[1 0 0.03977] ally's sound perception
  (Utilities|Casting|CastToBP_BaseSoldier Actor)
  (if (Utilities|Name|Equal(Name) _tag "Noise")
    (AI|Components|Blackboard|SetValueasBool (AI|GetBlackboard 0) (Utilities|Name|MakeLiteralName "Investigate") _bsuccessfullysensed)
    (AI|Components|Blackboard|SetValueasVector (AI|GetBlackboard 0) (Utilities|Name|MakeLiteralName "TargetLocation") _stimuluslocation)))

(event OnPerceptionUpdated(AIPerceptionSoldier)
  (params (UpdatedActors :type Array%20of%20Actor%20Object%20References))
  (for _array_element UpdatedActors
    ;[1 0 0.0231] target perception
    (bind _info (Class|AIPerceptionComponent|GetActorsPerception (Variables|Default|GetAIPerceptionSoldier) _array_element))
    (if (== (.target _info) (Game|GetPlayerCharacter 0))
      (for (_array_element_2 _array_index) (.lastsensedstimuli _info)
        (Variables|Default|SetSense _array_element_2)
        (switch int _array_index
          (:0
            ;[0 1 0.03028] Sense Sight
            (if (.bsuccessfullysensed (Variables|Default|GetSense)) :!label _label
              (AI|Components|Blackboard|SetValueasBool (AI|GetBlackboard 0) (Utilities|Name|MakeLiteralName "CanSeePlayer") (.bsuccessfullysensed (Variables|Default|GetSense)))
              (AI|Components|Blackboard|SetValueasBool (AI|GetBlackboard 0) (Utilities|Name|MakeLiteralName "Investigate") false)))
          (:1
            ;[1 0.9499 0] Sense Hearing
            (if (.bsuccessfullysensed (Variables|Default|GetSense))
              (AI|Components|Blackboard|SetValueasBool (AI|GetBlackboard 0) (Utilities|Name|MakeLiteralName "Investigate") (.bsuccessfullysensed (Variables|Default|GetSense)))
              (AI|Components|Blackboard|SetValueasVector (AI|GetBlackboard 0) (Utilities|Name|MakeLiteralName "TargetLocation") (.stimuluslocation (Variables|Default|GetSense)))))
          (:2
            ;[1 0 0.05677] Sense Damage
            (if (Utilities|Name|Equal(Name) (.tag (Variables|Default|GetSense)) "Noise")
              (AI|Components|Blackboard|SetValueasBool (AI|GetBlackboard 0) (Utilities|Name|MakeLiteralName "Investigate") (.bsuccessfullysensed (Variables|Default|GetSense)))
              (AI|Components|Blackboard|SetValueasVector (AI|GetBlackboard 0) (Utilities|Name|MakeLiteralName "TargetLocation") (.stimuluslocation (Variables|Default|GetSense)))
              (else
                (goto _label)))))))))

(event EventBeginPlay
  ;[1 0.1157 0] Random Behavior Tree
  (if (Math|Random|RandomBool)
    (AI|RunBehaviorTree "/Game/FpsStarterPack/System/AI/Treeandboard/BT_courageous.BT_courageous")
    (else
      (AI|RunBehaviorTree "/Game/FpsStarterPack/System/AI/Treeandboard/BT_ShootingCover.BT_ShootingCover"))))

(fn ConstructionScript)