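; Behavior tree task that has an AI soldier rise from cover and shoot for a few seconds.
; On execute it uncrouches the BP_BaseSoldier and starts its attack; a timer then stops the attack, crouches it and finishes successfully, while a dead soldier finishes immediately.
; Each tick sets the controller's focal point to the player's location.
; Abort uncrouches the soldier and sets its StopShooting flag.
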(event Custom|StopShooting
  (bind _bp_basesoldier (Variables|Default|GetBP_BaseSoldier))
  (Default|StopAttack _bp_basesoldier)
  (Character|Crouch _bp_basesoldier)
  (AI|BehaviorTree|FinishExecute true))

(event EventReceiveExecuteAI
  (params (OwnerController :type AI%20Controller%20Object%20Reference) (ControlledPawn :type Pawn%20Object%20Reference))
  (bind _asbp_base_soldier (Utilities|Casting|CastToBP_BaseSoldier ControlledPawn))
  (bind _output_get (Variables|Default|SetBP_BaseSoldier _asbp_base_soldier))
  (if (Variables|/Game/FpsStarterPack/System/AI/BP_BaseSoldier.BP_BaseSoldier_C|GetIsDead _asbp_base_soldier)
    (AI|BehaviorTree|FinishExecute true)
    (else
      (Character|UnCrouch _output_get)
      (Default|AIAttack (Variables|Default|GetBP_BaseSoldier))
      (Utilities|Time|SetTimerbyEvent (delegate Custom|StopShooting) 4.0))))

(event EventReceiveTickAI
  (params (OwnerController :type AI%20Controller%20Object%20Reference) (ControlledPawn :type Pawn%20Object%20Reference) (DeltaSeconds :type Float%20%28single-precision%29))
  (AI|SetFocalPoint OwnerController (Transformation|GetActorLocation (Game|GetPlayerCharacter 0))))

(event EventReceiveAbortAI
  (params (OwnerController :type AI%20Controller%20Object%20Reference) (ControlledPawn :type Pawn%20Object%20Reference))
  (bind _bp_basesoldier (Variables|Default|GetBP_BaseSoldier))
  (Character|UnCrouch _bp_basesoldier)
  (Variables|/Game/FpsStarterPack/System/AI/BP_BaseSoldier.BP_BaseSoldier_C|SetStopShooting _bp_basesoldier true)
  (Class|BTTaskBlueprintBase|FinishAbort))