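; Behavior Tree service that tracks how far an AI-controlled pawn is from its attack target.
; Each tick it reads the target actor from the blackboard, measures the distance between the two locations and writes it to the DistanceToTargetKey blackboard value.
; It also prints the distance as debug output, and an unconnected leftover holds a player-within-damage-range check.
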(event EventReceiveTickAI
  (params (OwnerController :type AI%20Controller%20Object%20Reference) (ControlledPawn :type Pawn%20Object%20Reference) (DeltaSeconds :type Float%20%28single-precision%29))
  (bind _returnvalue (Transformation|GetActorLocation ControlledPawn))
  (bind _attacktargetkey (Variables|Default|GetAttackTargetKey))
  (bind _returnvalue_2 (AI|BehaviorTree|GetBlackboardValueasActor _attacktargetkey))
  (bind _returnvalue_3 (Transformation|GetActorLocation _returnvalue_2))
  (bind _returnvalue_4 (Math|Vector|Distance(Vector) _returnvalue _returnvalue_3))
  (Development|PrintString (Utilities|String|ToString(Float) _returnvalue_4))
  (Class|BTFunctionLibrary|SetBlackboardValueasFloat (Variables|Default|GetDistanceToTargetKey) _returnvalue_4))

(event EventReceiveActivationAI
  (params (OwnerController :type AI%20Controller%20Object%20Reference) (ControlledPawn :type Pawn%20Object%20Reference)))