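; BP_SpawnAI is a spawner that keeps BP_BaseSoldier enemies coming while one or none remain in the level.
; Tick counts all soldiers and, when the count is low, waits through a short Delay before spawning one at a random point inside the BoxSpawn bounds.
; Each new soldier gets its default controller, is stored in Soldier, and has its AI focus set on the player character.
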(event EventTick
  (params (DeltaSeconds :type Float%20%28single-precision%29))
  (bind _boxspawn (Variables|Default|GetBoxSpawn))
  (bind (_origin _boxextent) (Collision|GetComponentBounds _boxspawn))
  (bind _outactors (Actor|GetAllActorsOfClass "/Game/FpsStarterPack/System/AI/BP_BaseSoldier.BP_BaseSoldier_C"))
  (if (<= (Utilities|Array|Length _outactors) 1)
    (Utilities|FlowControl|Delay 2.0)
    (bind _returnvalue (Game|SpawnActorfromClass :Class "/Game/FpsStarterPack/System/AI/BP_BaseSoldier.BP_BaseSoldier_C" :SpawnTransform (Math|Transform|MakeTransform (Math|Random|RandomPointinBoundingBox _origin _boxextent)) :CollisionHandlingOverride "Undefined" :TransformScaleMethod "MultiplyWithRoot" :Instigator 0))
    (Utilities|IsValid _returnvalue
      (:Is%20Valid
        (Pawn|SpawnDefaultController _returnvalue)
        (bind _output_get (Variables|Default|SetSoldier _returnvalue))
        (Utilities|IsValid _output_get
          (:Is%20Valid
            (AI|SetFocus (AI|GetAIController _output_get) (Game|GetPlayerCharacter 0))))))))

(fn ConstructionScript)